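; GI_Car_Game is the car game's Game Instance, adding and removing local players as input devices connect and disconnect.
; On Init it binds to input device connection changes.
; A connection creates a local player and calls ConnectToGame on its BPC_CarGame controller with the player index.
; A disconnection calls EnablePlayers on W_MainMenu and removes the last local player rather than matching the device.
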(event Custom|AddInput
  (params (NewConnectionState :type EInputDeviceConnectionState%20Enum :default "Invalid") (PlatformUserId :type Platform%20User%20Id%20Structure) (InputDeviceId :type Input%20Device%20Id%20Structure))
  (bind _returnvalue (Class|GameplayStatics|GetNumLocalPlayerControllers))
  (bind _returnvalue_2 (- _returnvalue 1))
  (bind _returnvalue_3 (Game|GetPlayerController _returnvalue_2))
  (switch Utilities|FlowControl|Switch|SwitchonEInputDeviceConnectionState NewConnectionState
    (:Disconnected
      (bind _foundwidgets (Widget|GetAllWidgetsOfClass "/Game/UI/W_MainMenu.W_MainMenu_C" false))
      (Default|EnablePlayers (Utilities|Array|Get(acopy) _foundwidgets))
      (Class|GameplayStatics|RemovePlayer _returnvalue_3 true)
      (Utilities|IsValid _returnvalue_3
        (:Is%20Valid
          (Actor|DestroyActor _returnvalue_3))))
    (:Connected
      (bind _returnvalue_4 (Class|GameplayStatics|CreatePlayer _returnvalue))
      (bind _asbpc_car_game (Utilities|Casting|CastToBPC_CarGame _returnvalue_4))
      (Default|ConnecttoGame _asbpc_car_game _returnvalue_2))))

(event EventInit
  (EventDispatchers|BindEventtoOnInputDeviceConnectionChange (delegate Custom|AddInput)))