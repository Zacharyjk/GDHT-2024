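; GM_Car_game is the car game's game mode, spawning local players and registering them with the game.
; Shortly after BeginPlay, it runs a loop sized by the connected input device count, calling CreatePlayer with automatic controller IDs.
; HandleStartingNewPlayer adds each new controller to PlayerList and passes the resulting index to BPC_CarGame's ConnectToGame.
; A minimum two-device check exists but is unused.
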(event Custom|Start%20Loading%20Players
  (bind _returnvalue (Class|InputDeviceLibrary|GetAllConnectedInputDevices))
  (if true
    (for _index (range 0 (- _returnvalue 1))
      (Class|GameplayStatics|CreatePlayer -1))))

(event EventBeginPlay
  (Utilities|FlowControl|DoOnce false
    (:Completed
      (Utilities|FlowControl|Delay 0.2)
      (CallFunction|StartLoadingPlayers))))

(event EventHandleStartingNewPlayer
  (params (NewPlayer :type Player%20Controller%20Object%20Reference))
  (bind _returnvalue (Utilities|Array|Add (Variables|Default|GetPlayer%20List) NewPlayer))
  (bind _asbpc_car_game (Utilities|Casting|CastToBPC_CarGame NewPlayer))
  (Default|ConnecttoGame _asbpc_car_game _returnvalue))

(fn ConstructionScript)